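; Game instance for Grapple Dash that keeps the player's best records across sessions: grapple points, best time, and best time on ground.
; On Init it loads the existing save slot, or creates a new Grapple_Dash_SAVE object if none exists.
; Save and load functions copy the records between instance variables and the save object; only saving writes to disk, and Init does not copy loaded values into the variables.
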(event `self.ReceiveInit`
  (bind _returnvalue (`GameplayStatics.DoesSaveGameExist` (`self.gi_saveSlotName`)))
  (if _returnvalue
    (bind _returnvalue_2 (`GameplayStatics.LoadGameFromSlot` (`self.gi_saveSlotName`)))
    (bind _asgrapple_dash_save (cast `/Game/Grapple_Dash/Blueprints/System/Grapple_Dash_SAVE` _returnvalue_2))
    (set `self.gi_saveGameData` _asgrapple_dash_save)
    (else
      (bind _returnvalue_3 (`GameplayStatics.CreateSaveGameObject` "/Game/Grapple_Dash/Blueprints/System/Grapple_Dash_SAVE.Grapple_Dash_SAVE_C"))
      (set `self.gi_saveGameData` _returnvalue_3))))

(fn `gi_loadPlayerData`
  (set `self.gi_bestTimeMinute` (`/Game/Grapple_Dash/Blueprints/System/Grapple_Dash_SAVE.sd_bestTimeMinute` (`self.gi_saveGameData`)))
  (set `self.gi_bestTimeSecond` (`/Game/Grapple_Dash/Blueprints/System/Grapple_Dash_SAVE.sd_bestTimeSecond` (`self.gi_saveGameData`)))
  (set `self.gi_bestGrapplePoints` (`/Game/Grapple_Dash/Blueprints/System/Grapple_Dash_SAVE.sd_bestGrapplePoints` (`self.gi_saveGameData`)))
  (set `self.gi_bestTimeOnGroundMinute` (`/Game/Grapple_Dash/Blueprints/System/Grapple_Dash_SAVE.sd_bestTimeOnGroundMinute` (`self.gi_saveGameData`)))
  (set `self.gi_bestTimeOnGroundSecond` (`/Game/Grapple_Dash/Blueprints/System/Grapple_Dash_SAVE.sd_bestTimeOnGroundSecond` (`self.gi_saveGameData`))))

(fn `gi_savePlayerData`
  (set `/Game/Grapple_Dash/Blueprints/System/Grapple_Dash_SAVE.sd_bestGrapplePoints` (`self.gi_bestGrapplePoints`) (`self.gi_saveGameData`))
  (set `/Game/Grapple_Dash/Blueprints/System/Grapple_Dash_SAVE.sd_bestTimeOnGroundMinute` (`self.gi_bestTimeOnGroundMinute`) (`self.gi_saveGameData`))
  (set `/Game/Grapple_Dash/Blueprints/System/Grapple_Dash_SAVE.sd_bestTimeOnGroundSecond` (`self.gi_bestTimeOnGroundSecond`) (`self.gi_saveGameData`))
  (set `/Game/Grapple_Dash/Blueprints/System/Grapple_Dash_SAVE.sd_bestTimeMinute` (`self.gi_bestTimeMinute`) (`self.gi_saveGameData`))
  (set `/Game/Grapple_Dash/Blueprints/System/Grapple_Dash_SAVE.sd_bestTimeSecond` (`self.gi_bestTimeSecond`) (`self.gi_saveGameData`))
  (`GameplayStatics.SaveGameToSlot` (`self.gi_saveGameData`) (`self.gi_saveSlotName`)))