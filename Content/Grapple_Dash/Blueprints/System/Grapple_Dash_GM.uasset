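; Game mode for Grapple Dash that tracks run stats and objective progress.
; Events count grapple point uses and collected objectives, activating the Victory_Ring_BP actor once all eight objectives are collected.
; Tick checks whether the player is moving on the ground, advancing minute/second timers for total time and, when grounded, time on the ground.
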(event `gm_grapplePointUsed`
  ;[0.5051 0.664 1 0.5] Count Grapple Points Used
  (bind _result (`/Engine/EditorBlueprintResources/StandardMacros.IncrementInt` (`self.gm_grapplePointsUsed`))
    (:`  `
      (set `self.gm_grapplePointsUsed` _result))))

(event `gm_objectiveCollected`
  ;[0.6882 0.4961 1 0.5] Count Objectives & Activate Victory Ring
  (bind _result (`/Engine/EditorBlueprintResources/StandardMacros.IncrementInt` (`self.gm_objectiveCount`))
    (:`  `
      (bind _output_get (set `self.gm_objectiveCount` (`KismetMathLibrary.Clamp` _result 0 8)))
      (if (== 8 _output_get)
        (bind _returnvalue (`GameplayStatics.GetActorOfClass` "/Game/Grapple_Dash/Blueprints/GameObjects/Victory_Ring_BP.Victory_Ring_BP_C"))
        (`/Game/Grapple_Dash/Blueprints/GameObjects/Victory_Ring_BP.wr_activate` _returnvalue)))))

(event `self.ReceiveTick`
  (params (DeltaSeconds :type "Float (single-precision)"))
  ;[0.4862 1 0.4456 0.5] Controls Score Timers
  (set `self.gm_deltaTime` DeltaSeconds)
  (bind _asplayer_bp (cast `/Game/Grapple_Dash/Blueprints/GameObjects/Player_BP` (`GameplayStatics.GetPlayerCharacter` 0)))
  (if (`NavMovementComponent.IsMovingOnGround` (`Character.CharacterMovement` _asplayer_bp))
    (`self.gm_calculateCurrentTimeOnGround`)
    (else
      (`self.gm_calculateCurrentTime`))))

(fn `gm_calculateCurrentTime`
  (bind _returnvalue (+ (`self.gm_deltaTime`) (`self.gm_currentSeconds`)))
  (if (>= _returnvalue 59.9)
    (bind _result (`/Engine/EditorBlueprintResources/StandardMacros.IncrementFloat` (`self.gm_currentMinutes`))
      (:`  `
        (set `self.gm_currentMinutes` _result)
        (set `self.gm_currentSeconds` 0.0)))
    (else
      (set `self.gm_currentSeconds` _returnvalue))))

(fn `gm_calculateCurrentTimeOnGround`
  (bind _returnvalue (+ (`self.gm_deltaTime`) (`self.gm_currentSecondsOnGround`)))
  (if (>= _returnvalue 59.9)
    (bind _result (`/Engine/EditorBlueprintResources/StandardMacros.IncrementFloat` (`self.gm_currentMinutesOnGround`))
      (:`  `
        (set `self.gm_currentMinutesOnGround` _result)
        (set `self.gm_currentSecondsOnGround` 0.0)
        (`self.gm_calculateCurrentTime`)))
    (else
      (set `self.gm_currentSecondsOnGround` _returnvalue)
      (`self.gm_calculateCurrentTime`))))

(fn `UserConstructionScript`)