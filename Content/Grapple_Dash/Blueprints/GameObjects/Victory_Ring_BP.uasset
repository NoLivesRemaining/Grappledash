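; Victory ring for Grapple Dash that becomes the win trigger once activated.
; The wr_activate event plays a timeline that fades the ring mesh's colour parameter from black to gold, then sets AllHoopsCollected when it finishes.
; An overlap on the collection collider, gated by that flag, clears all widgets and shows the Victory UI.
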(event `wr_activate`
  ;[0.2339 0.8497 1 0.5] Light up WinRing & enable collision
  (bind (_direction _alpha) (`Timeline|wr_activationTimeline`)
    (:`Update`
      (`MeshComponent.SetVectorParameterValueOnMaterials` (`self.wr_ringMesh_0`) "vr_colour" (`KismetMathLibrary.Conv_LinearColorToVector` (`KismetMathLibrary.LinearColorLerp` (struct) (struct :`R` 0.756863 :`G` 0.737255 :`B` 0.207843 :`A` 1.0) _alpha))))
    (:`Finished`
      (set `self.AllHoopsCollected` true))))

(event `self.wr_collectionCollider.OnComponentBeginOverlap`
  (params (OverlappedComponent :type "PrimitiveComponent Object Reference") (OtherActor :type "Actor Object Reference") (OtherComp :type "PrimitiveComponent Object Reference") (OtherBodyIndex :type Integer) (bFromSweep :type Boolean) (SweepResult :type "HitResult Structure (by ref)"))
  ;[0.5277 0.6176 1 0.5] Create Win UI on collision
  (if (`self.AllHoopsCollected`)
    (`WidgetLayoutLibrary.RemoveAllWidgets`)
    (bind _returnvalue (`|CreateWidget` "/Game/Grapple_Dash/Blueprints/UI/Victory_UI.Victory_UI_C"))
    (`UserWidget.AddToViewport` _returnvalue 0)))

(fn `UserConstructionScript`)