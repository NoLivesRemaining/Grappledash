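; Collectible objective ring for Grapple Dash that reports to the game mode when its collider is overlapped.
; On pickup it removes its collider and rotating movement, plays an attached power-down sound and fades the ring material from purple to black via a timeline.
; At begin play a scene capture is restricted to show only this actor, apparently for a UI render of the ring.
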(event `self.ReceiveBeginPlay`
  ;[0.945 0.5841 1 0.5] Refine gUI_ringRender
  (`SceneCaptureComponent.ShowOnlyActorComponents` (`self.or_sceneCaptureComponent2D`) self false))

(event `self.or_collectionCollider.OnComponentBeginOverlap`
  (params (OverlappedComponent :type "PrimitiveComponent Object Reference") (OtherActor :type "Actor Object Reference") (OtherComp :type "PrimitiveComponent Object Reference") (OtherBodyIndex :type Integer) (bFromSweep :type Boolean) (SweepResult :type "HitResult Structure (by ref)"))
  ;[0.6458 1 0.7782 0.5] Darken & stop ring movement when collected
  (bind _asgrapple_dash_gm (cast `/Game/Grapple_Dash/Blueprints/System/Grapple_Dash_GM` (`GameplayStatics.GetGameMode`)))
  (`/Game/Grapple_Dash/Blueprints/System/Grapple_Dash_GM.gm_objectiveCollected` _asgrapple_dash_gm)
  (`ActorComponent.K2_DestroyComponent` (`self.or_collectionCollider`))
  (`ActorComponent.K2_DestroyComponent` (`self.or_rotatingMovement`))
  (`GameplayStatics.SpawnSoundAttached` "/Game/Grapple_Dash/SFXAndMusic/RingPowerDown.RingPowerDown" (`self.or_ringMesh`) "None" (0.0 0.0 0.0) (struct) "KeepRelativeOffset" false 1.0 1.0 0.0 null null)
  (bind (_direction _alpha) (`Timeline|or_colourShiftToOffTimeline`)
    (:`Update`
      (`MeshComponent.SetVectorParameterValueOnMaterials` (`self.or_ringMesh`) "or_colour" (`KismetMathLibrary.Conv_LinearColorToVector` (`KismetMathLibrary.LinearColorLerp` (struct :`R` 0.571125 :`G` 0.177888 :`B` 0.760525 :`A` 1.0) (struct :`A` 1.0) _alpha))))))

(fn `UserConstructionScript`)