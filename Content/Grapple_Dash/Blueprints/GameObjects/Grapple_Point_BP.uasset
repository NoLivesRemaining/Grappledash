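; Grapple point actor that shifts colour and becomes temporarily ungrappleable after being hit by the grapple.
; The hit event runs a timeline that blends the mesh's material colour parameter from green to warning red.
; When that finishes, it clears the can-be-grappled flag and a second timeline fades the colour back to green.
; The flag is set again once the fade back completes.
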(event `g_hitByGrapple`
  (bind (_direction _alpha) (`Timeline|g_colourShiftToWarningTimeline` :!via `PlayFromStart`)
    (:`Update`
      (`MeshComponent.SetVectorParameterValueOnMaterials` (`self.g_grapplePointMesh`) "g_colour" (`KismetMathLibrary.Conv_LinearColorToVector` (`KismetMathLibrary.LinearColorLerp` (struct :`R` 0.192157 :`G` 0.756863 :`B` 0.454902 :`A` 1.0) (struct :`R` 0.756863 :`G` 0.188235 :`B` 0.176471 :`A` 1.0) _alpha))))
    (:`Finished`
      (set `self.g_canBeGrappled` false)
      (bind (_direction_2 _alpha_2) (`Timeline|g_colourShiftToNormalTimeline` :!via `PlayFromStart`)
        (:`Update`
          (`MeshComponent.SetVectorParameterValueOnMaterials` (`self.g_grapplePointMesh`) "g_colour" (`KismetMathLibrary.Conv_LinearColorToVector` (`KismetMathLibrary.LinearColorLerp` (struct :`R` 0.756863 :`G` 0.188235 :`B` 0.176471 :`A` 1.0) (struct :`R` 0.192157 :`G` 0.756863 :`B` 0.454902 :`A` 1.0) _alpha_2))))
        (:`Finished`
          (set `self.g_canBeGrappled` true))))))

(fn `UserConstructionScript`)